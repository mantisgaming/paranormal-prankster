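; BP_Spawner is a clickable actor that spawns a BP_Selectable when clicked.
; On click it spawns the selectable at a fixed hardcoded transform, passes it SpawnedItem as its SelectableItem, and calls that actor's SetMesh.
; Its construction script runs its own SetMesh, which applies a valid Model mesh and that mesh's first material to the Cube component.
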(event EventBeginPlay)

(event Collision|EventActorBeginOverlap
  (params (OtherActor :type Actor%20Object%20Reference)))

(event EventTick
  (params (DeltaSeconds :type Float%20%28single-precision%29)))

(event MouseInput|EventActorOnClicked
  (params (ButtonPressed :type Key%20Structure :default "None"))
  (bind _returnvalue (Game|SpawnActorfromClass "/Game/Blueprints/BP_Selectable.BP_Selectable_C" (Math|Transform|MakeTransform "-38.000000,73.000000,73.000000") "Undefined" "MultiplyWithRoot" 0 0))
  (Variables|/Game/Blueprints/BP_Selectable.BP_Selectable_C|SetSelectableItem _returnvalue (Variables|Default|GetSpawned%20Item))
  (Default|SetMesh _returnvalue))

(fn ConstructionScript
  (CallFunction|SetMesh))

(fn SetMesh
  (bind _cube (Variables|Default|GetCube))
  (bind _model (Variables|Default|GetModel)
    (:then
      (Components|StaticMesh|SetStaticMesh _cube _model)
      (Rendering|Material|SetMaterial _cube 0 (Rendering|Material|GetMaterial _model 0)))
    (:else)))